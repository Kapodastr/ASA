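; BP_EnemyLaser is a laser projectile, named for enemy fire, that resolves impacts in its Hit event.
; Physics-simulating components receive a velocity-based impulse; otherwise it branches on collision object type.
; Pawns take point damage of type PlayerDamage, multiplied for "head" bone hits (with a debug print), while Destructibles take generic damage.
; It destroys itself after these impacts and on World Static or Dynamic hits.
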(event `self.ReceiveHit`
  (params (MyComp :type "PrimitiveComponent Object Reference") (Other :type "Actor Object Reference") (OtherComp :type "PrimitiveComponent Object Reference") (bSelfMoved :type Boolean) (HitLocation :type "Vector Structure") (HitNormal :type "Vector Structure") (NormalImpulse :type "Vector Structure") (Hit :type "HitResult Structure (by ref)"))
  (bind _returnvalue (`self.K2_GetActorLocation`))
  (bind _hitactor (`self.HitActor`))
  (bind _basedamage (`self.BaseDamage`))
  (bind _returnvalue_2 (== (`KismetStringLibrary.Conv_NameToString` (`.HitBoneName` (`GameplayStatics.BreakHitResult` Hit))) "head"))
  (set `self.HitActor` Other)
  (bind _output_get (set `self.HitComp` OtherComp))
  (if (`KismetSystemLibrary.IsValid` _output_get)
    (if (`SceneComponent.IsSimulatingPhysics` (`self.HitComp`) "None")
      (`PrimitiveComponent.AddImpulseAtLocation` (`self.HitComp`) (* (`self.GetVelocity`) 8.0) _returnvalue "None")
      (`self.K2_DestroyActor` :!label _label) ; Then destroy this projectile
      (else
        (switch `ECollisionChannel` (`PrimitiveComponent.GetCollisionObjectType` OtherComp)
          (:`ECC_WorldStatic`
            _)
          (:`ECC_WorldDynamic`
            _)
          (:`ECC_Pawn`
            (`KismetSystemLibrary.PrintString` (`KismetStringLibrary.Conv_BoolToString` _returnvalue_2))
            (if _returnvalue_2
              (`GameplayStatics.ApplyPointDamage` _hitactor (* _basedamage (`self.CritMultiplier`)) _returnvalue Hit null null "/Game/ASAP/Weapon/PlayerDamage.PlayerDamage_C")
              (goto _label)
              (else
                (`GameplayStatics.ApplyPointDamage` _hitactor _basedamage _returnvalue Hit null null "/Game/ASAP/Weapon/PlayerDamage.PlayerDamage_C")
                (goto _label))))
          (:`ECC_Destructible`
            (`GameplayStatics.ApplyDamage` _hitactor _basedamage)
            (goto _label)))
        (`self.K2_DestroyActor`)))))

(fn `UserConstructionScript`)